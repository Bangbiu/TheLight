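; Interactive campfire Blueprint that ties the playback speed of its Fire to the Luminance value.
; Two seconds after BeginPlay it sets the Fire's CustomTimeDilation to zero, freezing it.
; Illuminate and FadeDelta call their parent versions, then copy Luminance into that time dilation, so the fire's animation speed follows the illumination and fade.
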(event `self.ReceiveBeginPlay`
  (`KismetSystemLibrary.Delay` 2.0)
  (set `ParticleSystemComponent.CustomTimeDilation` 0.0 (`self.Fire`)))

(event `self.Illuminate`
  (`parent.Illuminate`)
  (set `ParticleSystemComponent.CustomTimeDilation` (`self.Luminance`) (`self.Fire`) :!label _label))

(event `self.FadeDelta`
  (`parent.FadeDelta`)
  (goto _label))

(fn `UserConstructionScript`
  (`parent.UserConstructionScript`))