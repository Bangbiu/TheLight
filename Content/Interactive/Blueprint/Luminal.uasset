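; Luminal is a selectable, illuminable light object that drives an outline highlight and a point light.
; Selection events toggle the outline, while Illuminate sets full fade and changes state.
; FadeDelta decays Luminance, boosted by nearby Luminals in that same state, updates outline and intensity, and clears its timer at the range limit.
; The light-up timeline that would start this looping timer is disconnected, so it never runs.
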(event `self.ReceiveBeginPlay`)

(event `UnSelect Luminal`
  (`/Game/BP/LightOutline_Item.OnSelectCancel` (`self.LightOutline_Item`)))

(event `Select On Luminal`
  (`/Game/BP/LightOutline_Item.OnSelectItem` (`self.LightOutline_Item`)))

(event `Illuminate`
  (`/Game/BP/LightOutline_Item.OnFade` (`self.LightOutline_Item`) 1.0)
  (set `self.State` "NewEnumerator3"))

(event `FadeDelta`
  (bind _luminance (`self.Luminance`))
  (bind _out (`/Game/Data/GeneralFunctions.Actor In Radial Range` self "Luminal_C" (`self.ResonateBound`)))
  (for _array_element _out
    (if (`|EnumEquality` (`/Game/Interactive/Blueprint/Luminal.State` (cast `/Game/Interactive/Blueprint/Luminal` _array_element :!pure true)) "NewEnumerator3")
      (`/Game/Data/GeneralFunctions.OffsetInPercentRange` (`self.Luminance`) 0.05)))
  (bind _reachbottom (`/Game/Data/GeneralFunctions.OffsetInPercentRange` (`self.Luminance`) -0.01))
  (`self.SetFadeProgress` _luminance)
  (`self.SetLightIntensity` _luminance)
  (if _reachbottom
    (set `self.State` "NewEnumerator1")
    (`KismetSystemLibrary.K2_ClearAndInvalidateTimerHandle` (`self.FadeHandle`))))

(fn `SetFadeProgress`
  (params (Progress :type "Float (double-precision)"))
  (`/Game/BP/LightOutline_Item.OnFade` (`self.LightOutline_Item`) (`KismetMathLibrary.Lerp` -0.5 1.5 Progress)))

(fn `SetLightIntensity`
  (params (Progress :type "Float (double-precision)"))
  (`LightComponent.SetIntensity` (`self.PointLight`) (`KismetMathLibrary.Lerp` 0.0 3000.0 (`KismetMathLibrary.FClamp` (- Progress 0.1)))))

(fn `UserConstructionScript`)

(fn `VaryCoutourDelta`)